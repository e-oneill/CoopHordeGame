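; Player character Blueprint that layers HUD and first-level weapon animation over inherited fire, reload and zoom functions.
; On BeginPlay it binds health changes and creates crosshair, HUD and health widgets for the local player, removing health and ammo UI after death.
; Input events call the weapon functions and play montages from the current weapon's GunAnimationPack, switching between hip and ironsight poses.
; Weapon switches re-enter the BeginPlay hip-pose setup.
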(event `UI-OnHealthChanged`
  (params (HealthComp :type "SHealthComponent Object Reference") (Health :type "Float (double-precision)") (HealthDelta :type "Float (double-precision)") (DamageType :type "DamageType Object Reference") (InstigatedBy :type "Controller Object Reference") (DamageCauser :type "Actor Object Reference"))
  (bind _target (`self.Target`))
  (`/Engine/EditorBlueprintResources/StandardMacros.IsValid` _target
    (:`Is Valid`
      (if (and (<= Health 0.0) (not (`SCharacter.bDied` _target)))
        (`KismetSystemLibrary.Delay` 2.0)
        (`|ExecutionSequence`
          (:`then_0`
            (`Widget.RemoveFromParent` (`self.HealthUIIndicator`)))
          (:`then_1`
            (`Widget.RemoveFromParent` (`self.AmmoUI`))))))))

(event `self.ReceiveEndPlay`
  (params (EndPlayReason :type "EEndPlayReason Enum" :default "Destroyed"))
  (`Widget.RemoveFromParent` (`/Game/UI/WBP_PlayerHud.WBP_Minimap_1` (stale `self.ReceiveBeginPlay` _returnvalue_2))))

(event `self.ReceiveBeginPlay`
  (bind _currentweapon (`self.CurrentWeapon`))
  ;[1 1 1] UI Init
  (set `self.Tags` (`|MakeArray` "Player" :!type "Name"))
  (`|ExecutionSequence`
    (:`then_0`
      (add `SHealthComponent.OnHealthChanged` (`self.HealthComponent`) (delegate `UI-OnHealthChanged`)))
    (:`then_1`
      (if (`self.IsLocallyControlled`)
        (`|ExecutionSequence`
          (:`then_0`
            (bind _returnvalue (`|CreateWidget` "/Game/UI/WBP_Crosshair.WBP_Crosshair_C"))
            (`UserWidget.AddToViewport` _returnvalue 0)
            (bind _returnvalue_2 (`|CreateWidget` "/Game/UI/WBP_PlayerHud.WBP_PlayerHud_C"))
            (`UserWidget.AddToViewport` _returnvalue_2 0)
            (set `self.AmmoUI` _returnvalue_2))
          (:`then_1`
            (bind _returnvalue_3 (`|CreateWidget` "/Game/UI/WBP_HealthLogoIndicator.WBP_HealthLogoIndicator_C"))
            (`UserWidget.AddToViewport` _returnvalue_3 0)
            (set `self.HealthUIIndicator` _returnvalue_3)))))
    (:`then_2`
      (`KismetSystemLibrary.Delay` 0.2)
      (`/Engine/EditorBlueprintResources/StandardMacros.IsValid` _currentweapon :!label _label
        (:`Is Valid`
          _)
        (:`Is Not Valid`
          (`KismetSystemLibrary.Delay` 1.0)))
      (`self.PlayAnimMontage` (`SGunAnimationPack.HipAnimation` (`SRangedWeapon.GunAnimationPack` _currentweapon)) 0.0))))

(event `self.OnSwitchWeapon`
  ;[1 1 1] UI Init
  (goto _label))

(event `InputAction|Reload`
  (params (Key :type "Key Structure"))
  (bind _currentweapon (`self.CurrentWeapon`))
  (bind _gunanimationpack (`SRangedWeapon.GunAnimationPack` _currentweapon))
  ;[1 1 1] Comment
  (:`Pressed`
    (if (< (`self.CurrentAmmo`) (`self.DefaultAmmo`))
      (set `self.bAimDownSights` false)
      (bind _returnvalue (`self.PlayAnimMontage` (`SGunAnimationPack.Reload` _gunanimationpack)))
      (`self.StartReload`)
      (`GameplayStatics.PlaySoundAtLocation` "/Game/Warfare_SFX_Bundle/Gun_Sound_Essentials/Cues/Reload_03_Cue.Reload_03_Cue" (`self.K2_GetActorLocation` _currentweapon) (struct) 1.0 1.0 0.0 null null null)
      (`KismetSystemLibrary.Delay` (- _returnvalue 0.25))
      (`self.PlayAnimMontage` (`SGunAnimationPack.HipAnimation` _gunanimationpack)))))

(event `InputAction|SwitchWeapon`
  (params (Key :type "Key Structure")))

(event `InputAction|AimDownSights`
  (params (Key :type "Key Structure"))
  (bind _gunanimationpack (`SRangedWeapon.GunAnimationPack` (`self.CurrentWeapon`)))
  (bind _ironsights (`SGunAnimationPack.Ironsights` _gunanimationpack))
  ;[1 1 1] AIm Down Sights
  (:`Pressed`
    (`self.BeginZoom`)
    (`self.PlayAnimMontage` _ironsights)
    (set `self.bAimDownSights` true))
  (:`Released`
    (`self.EndZoom`)
    (`self.StopAnimMontage` _ironsights)
    (`self.PlayAnimMontage` (`SGunAnimationPack.HipAnimation` _gunanimationpack))
    (set `self.bAimDownSights` false)))

(event `InputAction|Fire`
  (params (Key :type "Key Structure"))
  (bind _gunanimationpack (`SRangedWeapon.GunAnimationPack` (`self.CurrentWeapon`)))
  (bind _ironsights (`SGunAnimationPack.Ironsights` _gunanimationpack))
  (:`Pressed`
    (`self.StartFire`)
    (if (`self.bAimDownSights`)
      (`self.PlayAnimMontage` (`SGunAnimationPack.IronsightsFire` _gunanimationpack))
      (`self.PlayAnimMontage` _ironsights 0.0)
      (else
        (`self.PlayAnimMontage` (`SGunAnimationPack.Fire` _gunanimationpack)))))
  (:`Released`
    (`self.StopFire`)
    (if (`self.bAimDownSights`)
      (`self.PlayAnimMontage` _ironsights))))

(fn `UserConstructionScript`)