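; Game state Blueprint that drives the wave status HUD and the countdown between waves.
; On BeginPlay, after a short delay, it finds the locally controlled player-tagged character and shows a wave state widget.
; WaveStateChanged resets the timer from the game mode on the authority, removes the widget shortly into a wave and recreates it on completion.
; An authority-only Tick uses Delay to decrement Seconds about once per second.
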(event `self.ReceiveBeginPlay`
  (`KismetSystemLibrary.Delay` 0.2)
  (bind _outactors (`GameplayStatics.GetAllActorsOfClassWithTag` "/Script/CoopHordeGame.SCharacter" "Player"))
  (for _array_element _outactors
    (bind _returnvalue (`Pawn.GetController` _array_element))
    (`/Engine/EditorBlueprintResources/StandardMacros.IsValid` _returnvalue
      (:`Is Valid`
        (if (`Controller.IsLocalPlayerController` _returnvalue)
          (set `self.LocalCharacter` _array_element)
          (cast `PlayerController` _returnvalue)
          (bind _returnvalue_2 (`|CreateWidget` "/Game/UI/WBP_WaveState.WBP_WaveState_C" :!label _label))
          (`UserWidget.AddToViewport` _returnvalue_2 0))))))

(event `self.WaveStateChanged`
  (params (NewState :type "EWaveState Enum" :default "WaitingToStart") (OldState :type "EWaveState Enum" :default "WaitingToStart"))
  (switch `EWaveState` (`self.WaveState`)
    (:`WaitingToStart`
      (if (`self.HasAuthority`)
        (bind _asbp_test_game_mode (cast `/Game/Blueprints/GameState/BP_TEST_GameMode` (`GameplayStatics.GetGameMode`)))
        (set `self.seconds` (`SGameMode.GetTimeBetweenWaves` _asbp_test_game_mode))))
    (:`WaveInProgress`
      (`KismetSystemLibrary.Delay` 5.0)
      (`Widget.RemoveFromParent` (stale `self.ReceiveBeginPlay` _returnvalue_2)))
    (:`WaveComplete`
      (goto _label))))

(event `self.ReceiveTick`
  (params (DeltaSeconds :type "Float (single-precision)"))
  (bind _seconds (`self.seconds`))
  (if (and (> _seconds 0.0) (`self.HasAuthority`))
    (`KismetSystemLibrary.Delay` 1.0)
    (`/Engine/EditorBlueprintResources/StandardMacros.DecrementFloat` _seconds)))

(fn `UserConstructionScript`)