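; Test game mode that spawns AI bots and awards score to players for killing them.
; SpawnNewBot runs an EQS query (random best 25%) and spawns a bot at each returned location, with a random roll that effectively always picks BP_AdvancedAi over BP_TrackerBot.
; A kill delegate bound on BeginPlay adds score to the SPlayerState when a player-owned killer eliminates a non-player pawn, then prints the total.
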(event `self.SpawnNewBot`
  (bind _returnvalue (`EnvQueryManager.RunEQSQuery` "/Game/Blueprints/AI/EQS_FindSpawnLocation.EQS_FindSpawnLocation" self "RandomBest25Pct"))
  (add `EnvQueryInstanceBlueprintWrapper.OnQueryFinishedEvent` _returnvalue (delegate `OnQueryFinishedEvent_Event_0`)))

(event `OnQueryFinishedEvent_Event_0`
  (params (QueryInstance :type "EnvQueryInstanceBlueprintWrapper Object Reference") (QueryStatus :type "EEnvQueryStatus Enum" :default "Processing"))
  (switch `EEnvQueryStatus` QueryStatus
    (:`Success`
      (bind _resultlocations (`EnvQueryInstanceBlueprintWrapper.GetQueryResultsAsLocations` QueryInstance))
      (for _array_element _resultlocations
        (`|SpawnActorFromClass` (select `bool` (<= (`KismetMathLibrary.RandomFloatInRange` 0.0 100.0) 100.0) :`false` "/Game/Blueprints/NPCs/BP_TrackerBot.BP_TrackerBot_C" :`true` "/Game/Blueprints/AI/AdvancedAI/BP_AdvancedAi.BP_AdvancedAi_C" :!type "Actor Class Reference") (`KismetMathLibrary.MakeTransform` _array_element) "AdjustIfPossibleButDontSpawnIfColliding" "OverrideRootScale" null null)))))

(event `self.ReceiveBeginPlay`
  (add `self.OnActorKilled` (delegate `ActorKilledCustom`)))

(event `ActorKilledCustom` :!signature `self.OnActorKilled`
  (params (VictimActor :type "Actor Object Reference") (KillerActor :type "Actor Object Reference"))
  (bind _aspawn (cast `Pawn` VictimActor))
  (if (not (`Pawn.IsPlayerControlled` _aspawn))
    (bind _aspawn_2 (cast `Pawn` (`self.GetOwner` KillerActor)))
    (if (`Pawn.IsPlayerControlled` _aspawn_2)
      (bind _assplayer_state (cast `SPlayerState` (`Pawn.PlayerState` _aspawn_2)))
      (`SPlayerState.AddScore` _assplayer_state 20.0)
      (`KismetSystemLibrary.PrintString` (`KismetStringLibrary.Conv_DoubleToString` (`PlayerState.Score` _assplayer_state))))))

(fn `UserConstructionScript`)