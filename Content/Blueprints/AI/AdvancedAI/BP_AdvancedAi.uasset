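; AI-controlled actor that starts the BT_AdvancedAI behavior tree through its AI controller on BeginPlay.
; It has an AIPerception component, but the target perception update handler is empty.
; Logic that would write the player pawn to the TargetActor blackboard key is disconnected and never runs.
; CheckForPlayerInLOS is an empty stub, so this Blueprint performs no player detection itself.
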(event `self.ReceiveBeginPlay`
  (bind _returnvalue (`AIBlueprintHelperLibrary.GetAIController` self))
  (`/Engine/EditorBlueprintResources/StandardMacros.IsValid` _returnvalue
    (:`Is Valid`
      (`AIController.RunBehaviorTree` _returnvalue "/Game/Blueprints/AI/AdvancedAI/BT_AdvancedAI.BT_AdvancedAI"))))

(event `self.ReceiveTick`
  (params (DeltaSeconds :type "Float (single-precision)")))

(event `self.AIPerception.OnTargetPerceptionUpdated`
  (params (Actor :type "Actor Object Reference") (Stimulus :type "AIStimulus Structure")))

(fn `CheckForPlayerInLOS`)

(fn `UserConstructionScript`)