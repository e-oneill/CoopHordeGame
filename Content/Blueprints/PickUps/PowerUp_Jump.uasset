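; Jump power-up pickup that temporarily boosts the activating character's jump velocity and air control.
; On a state change it sets mesh visibility opposite to the active flag, silences its loop audio and plays a pickup sound.
; The activator event stores the character and multiplies both movement values.
; On expiry it divides them by the same factors to undo the boost, then destroys itself.
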(event `self.OnPowerUpStateChanged`
  (params (bNewIsActive :type Boolean))
  (`SceneComponent.SetVisibility` (`self.StaticMesh`) (not bNewIsActive) true)
  (`AudioComponent.SetVolumeMultiplier` (`self.powerup_loop_01`) 0.0)
  (`GameplayStatics.PlaySoundAtLocation` "/Game/Blueprints/PickUps/Powerups/Pickup_powerup_Cue.Pickup_powerup_Cue" (`self.K2_GetActorLocation`) (struct) 1.0 1.0 0.0 null null null))

(event `self.OnPowerUpHasActivator`
  (params (NewActivator :type "SCharacter Object Reference"))
  (bind _output_get (set `self.New Activator` NewActivator))
  (bind _charactermovement (`Character.CharacterMovement` _output_get))
  (set `CharacterMovementComponent.JumpZVelocity` (* 1.5 (`CharacterMovementComponent.JumpZVelocity` _charactermovement)) _charactermovement)
  (set `CharacterMovementComponent.AirControl` (* 5.0 (`CharacterMovementComponent.AirControl` _charactermovement)) _charactermovement))

(event `self.ReceiveBeginPlay`)

(event `self.OnExpired`
  (bind _charactermovement (`Character.CharacterMovement` (stale `self.OnPowerUpHasActivator` _output_get)))
  (set `CharacterMovementComponent.JumpZVelocity` (/ (`CharacterMovementComponent.JumpZVelocity` _charactermovement) 1.5) _charactermovement)
  (set `CharacterMovementComponent.AirControl` (/ (`CharacterMovementComponent.AirControl` _charactermovement) 5.0) _charactermovement)
  (`self.K2_DestroyActor`))

(fn `UserConstructionScript`)