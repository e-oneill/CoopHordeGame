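; A power-up pickup that temporarily doubles the movement speed of every SCharacter in the world.
; On state change it toggles mesh visibility, mutes its loop audio and plays a pickup sound.
; Activation doubles each character's MaxWalkSpeed from its current max speed; expiry halves it rather than restoring a saved value.
; DestroyActor is called inside the expiry loop body.
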(event `self.OnPowerUpStateChanged`
  (params (bNewIsActive :type Boolean))
  (`SceneComponent.SetVisibility` (`self.StaticMesh`) (not bNewIsActive) true)
  (`AudioComponent.SetVolumeMultiplier` (`self.powerup_loop_01`) 0.0)
  (`GameplayStatics.PlaySoundAtLocation` "/Game/Blueprints/PickUps/Powerups/Pickup_powerup_Cue.Pickup_powerup_Cue" (`self.K2_GetActorLocation`) (struct) 1.0 1.0 0.0 null null null))

(event `self.OnPowerUpHasActivator`
  (params (NewActivator :type "SCharacter Object Reference"))
  (bind _outactors (`GameplayStatics.GetAllActorsOfClass` "/Script/CoopHordeGame.SCharacter"))
  (for _array_element _outactors
    (bind _returnvalue (`self.GetComponentByClass` _array_element "/Script/Engine.CharacterMovementComponent"))
    (set `CharacterMovementComponent.MaxWalkSpeed` (* 2.0 (`MovementComponent.GetMaxSpeed` _returnvalue)) _returnvalue)))

(event `self.ReceiveBeginPlay`)

(event `self.OnExpired`
  (bind _outactors (`GameplayStatics.GetAllActorsOfClass` "/Script/CoopHordeGame.SCharacter"))
  (for _array_element _outactors
    (bind _returnvalue (`self.GetComponentByClass` _array_element "/Script/Engine.CharacterMovementComponent"))
    (set `CharacterMovementComponent.MaxWalkSpeed` (/ (`MovementComponent.GetMaxSpeed` _returnvalue) 2.0) _returnvalue)
    (`self.K2_DestroyActor`)))

(fn `UserConstructionScript`)