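; Infinite ammo power-up pickup that temporarily grants unlimited ammo to the actor that activates it.
; Power-up state changes set the mesh visibility opposite to the active state, mute the looping sound and play a pickup cue.
; The activator event stores the actor and sets its infinite ammo flag, which expiry clears before destroying the pickup.
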(event `self.OnPowerUpStateChanged`
  (params (bNewIsActive :type Boolean))
  (`SceneComponent.SetVisibility` (`self.StaticMesh`) (not bNewIsActive) true)
  (`AudioComponent.SetVolumeMultiplier` (`self.powerup_loop_01`) 0.0)
  (`GameplayStatics.PlaySoundAtLocation` "/Game/Blueprints/PickUps/Powerups/Pickup_powerup_Cue.Pickup_powerup_Cue" (`self.K2_GetActorLocation`) (struct) 1.0 1.0 0.0 null null null))

(event `self.OnPowerUpHasActivator`
  (params (NewActivator :type "SCharacter Object Reference"))
  (bind _output_get (set `self.New Activator` NewActivator))
  (set `SCharacter.bHasInfiniteAmmo` true _output_get))

(event `self.ReceiveBeginPlay`)

(event `self.OnExpired`
  (set `SCharacter.bHasInfiniteAmmo` false (`self.New Activator`))
  (`self.K2_DestroyActor`))

(fn `UserConstructionScript`)