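; A health regeneration power-up pickup that heals every SCharacter in the level by HealAmount on each power-up tick.
; Each tick gathers all SCharacter actors and calls Heal on their SHealthComponent, rather than targeting only one player.
; A state change sets mesh visibility opposite to the active state, mutes the loop audio and plays the pickup sound.
; The actor destroys itself on expiry.
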(event `self.OnPowerUpStateChanged`
  (params (bNewIsActive :type Boolean))
  (`SceneComponent.SetVisibility` (`self.StaticMesh`) (not bNewIsActive) true)
  (`AudioComponent.SetVolumeMultiplier` (`self.powerup_loop_01`) 0.0)
  (`GameplayStatics.PlaySoundAtLocation` "/Game/Blueprints/PickUps/Powerups/Pickup_powerup_Cue.Pickup_powerup_Cue" (`self.K2_GetActorLocation`) (struct) 1.0 1.0 0.0 null null null))

(event `self.OnExpired`
  (`self.K2_DestroyActor`))

(event `self.OnActivated`)

(event `self.ReceiveBeginPlay`)

(event `self.OnPowerUpTicked`
  ;[1 1 1] Handle Tick Effect
  (bind _outactors (`GameplayStatics.GetAllActorsOfClass` "/Script/CoopHordeGame.SCharacter"))
  (for _array_element _outactors
    (`/Engine/EditorBlueprintResources/StandardMacros.IsValid` _array_element
      (:`Is Valid`
        (`SHealthComponent.Heal` (`self.GetComponentByClass` _array_element "/Script/CoopHordeGame.SHealthComponent") (`self.Heal Amount`))))))

(fn `UserConstructionScript`)